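; BP_Barrackade is a damageable barricade building built on a destructible cube mesh.
; Its Hurt event subtracts damage from Health and briefly swaps in a hurt material, restoring the original cached by the construction script if it survives.
; At zero health it applies radius damage to its destructible mesh, disables actor collision, calls the dead dispatch and destroys itself after a delay.
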(event `self.Hurt`
  (params (Damage :type "Float (single-precision)"))
  (bind _output_get (set `self.Health` (- (`self.Health`) Damage)))
  (`PrimitiveComponent.SetMaterial` (`self.DestructibleCube_DM`) 0 (`self.HurtMaterial`))
  (if (<= _output_get 0.0)
    (`DestructibleComponent.ApplyRadiusDamage` (`self.DestructibleCube_DM`) 5.0 (`self.K2_GetActorLocation`) 10.0 10.0 false)
    (`self.SetActorEnableCollision` false)
    (`self.DeadDispatch`)
    (`KismetSystemLibrary.Delay` 20.0)
    (`self.K2_DestroyActor`)
    (else
      (`KismetSystemLibrary.Delay` 0.1)
      (`PrimitiveComponent.SetMaterial` (`self.DestructibleCube_DM`) 0 (`self.Original Building Material`)))))

(fn `UserConstructionScript`
  (`parent.UserConstructionScript`)
  (set `self.Original Building Material` (`PrimitiveComponent.GetMaterial` (`self.DestructibleCube_DM`) 0)))