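; Base turret actor assembled from separate head, body and nozzle part actors.
; BeginPlay spawns the parent class of each part, attaches it to its matching component and passes the turret as owner reference.
; Setters swap parts by destroying the old actor, then attaching and re-parenting the new one.
; HurtTurret sets Health to Damage minus Health (operands appear reversed) and calls Kill at zero or below, destroying all parts and the turret.
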(event `self.ReceiveBeginPlay`
  (`self.Initialize`))

(fn `HurtTurret`
  (params (Damage :type "Float (double-precision)"))
  (bind _output_get (set `self.Health` (- Damage (`self.Health`))))
  (if (<= _output_get 0.0)
    (`self.Kill`)))

(fn `Initialize`
  (bind _returnvalue (`|SpawnActorFromClass` "/Game/Game/Turret/Heads/BP_Parent_Head.BP_Parent_Head_C" (`KismetMathLibrary.MakeTransform` (0.0 0.0 0.0)) "Undefined" "OverrideRootScale" null self))
  (bind _output_get (set `self.HeadActor` _returnvalue))
  (`self.K2_AttachToComponent` _output_get (`self.Head`) "None" "KeepRelative" "KeepRelative" "KeepRelative" true)
  (bind _returnvalue_2 (`|SpawnActorFromClass` "/Game/Game/Turret/Bodys/BP_Parent_Body.BP_Parent_Body_C" (`KismetMathLibrary.MakeTransform` (0.0 0.0 0.0)) "Undefined" "OverrideRootScale" null self))
  (bind _output_get_2 (set `self.BodyActor` _returnvalue_2))
  (`self.K2_AttachToComponent` _output_get_2 (`self.Body`) "None" "KeepRelative" "KeepRelative" "KeepRelative" true)
  (bind _returnvalue_3 (`|SpawnActorFromClass` "/Game/Game/Turret/Nozzle/BP_Parent_Nozzle.BP_Parent_Nozzle_C" (`KismetMathLibrary.MakeTransform` (0.0 0.0 0.0)) "Undefined" "OverrideRootScale" null "/Game/Main/Shapes/DestructibleCube.DestructibleCube" 0 self))
  (bind _output_get_3 (set `self.NozzleActor` _returnvalue_3))
  (`self.K2_AttachToComponent` _output_get_3 (`self.Nozzle`) "None" "KeepRelative" "KeepRelative" "KeepRelative" true))

(fn `Kill`
  (`self.K2_DestroyActor` (`self.HeadActor`))
  (`self.K2_DestroyActor` (`self.BodyActor`))
  (`self.K2_DestroyActor` (`self.NozzleActor`))
  (`self.K2_DestroyActor`))

(fn `SetBodyActor`
  (params (`New Body` :type "/Game/Game/Turret/Bodys/BP_Parent_Body Object Reference"))
  (`/Engine/EditorBlueprintResources/StandardMacros.IsValid` (`self.BodyActor`)
    (:`Is Valid`
      (if (not (== (`self.BodyActor`) `New Body`))
        (`self.K2_DestroyActor` (`self.BodyActor`))
        (bind _output_get (set `self.BodyActor` `New Body` :!label _label))
        (`self.K2_AttachToComponent` _output_get (`self.Body`) "None" "KeepRelative" "KeepRelative" "KeepRelative" true)
        (`/Game/Game/Turret/BP_TurretSection.Set Parent Turret` (`self.BodyActor`) self)))
    (:`Is Not Valid`
      (goto _label))))

(fn `SetHeadActor`
  (params (`New Head` :type "/Game/Game/Turret/Heads/BP_Parent_Head Object Reference"))
  (`/Engine/EditorBlueprintResources/StandardMacros.IsValid` (`self.HeadActor`)
    (:`Is Valid`
      (if (not (== (`self.HeadActor`) `New Head`))
        (`self.K2_DestroyActor` (`self.HeadActor`))
        (bind _output_get (set `self.HeadActor` `New Head` :!label _label))
        (`self.K2_AttachToComponent` _output_get (`self.Head`) "None" "KeepRelative" "KeepRelative" "KeepRelative" true)
        (`/Game/Game/Turret/BP_TurretSection.Set Parent Turret` (`self.HeadActor`) self)))
    (:`Is Not Valid`
      (goto _label))))

(fn `SetNozzleActor`
  (params (`New Nozzle` :type "/Game/Game/Turret/Nozzle/BP_Parent_Nozzle Object Reference"))
  (`/Engine/EditorBlueprintResources/StandardMacros.IsValid` (`self.NozzleActor`)
    (:`Is Valid`
      (if (not (== (`self.NozzleActor`) `New Nozzle`))
        (`self.K2_DestroyActor` (`self.NozzleActor`))
        (bind _output_get (set `self.NozzleActor` `New Nozzle` :!label _label))
        (`self.K2_AttachToComponent` _output_get (`self.Nozzle`) "None" "KeepRelative" "KeepRelative" "KeepRelative" true)
        (`/Game/Game/Turret/BP_TurretSection.Set Parent Turret` (`self.NozzleActor`) self)))
    (:`Is Not Valid`
      (goto _label))))

(fn `UserConstructionScript`)