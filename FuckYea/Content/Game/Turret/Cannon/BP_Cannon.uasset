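; BP_Cannon is a cannon turret that picks targets within its reach and can be destroyed by damage.
; Overlaps on ReachRadius pass the entering actor to its Cannon_Controller AI as the target.
; When an actor leaves, the controller empties that target and takes the first actor still overlapping, with no filtering in this graph.
; HurtTurret subtracts damage from Health and calls Kill at zero or below.
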(event `self.ReachRadius.OnComponentBeginOverlap`
  (params (OverlappedComponent :type "PrimitiveComponent Object Reference") (OtherActor :type "Actor Object Reference") (OtherComp :type "PrimitiveComponent Object Reference") (OtherBodyIndex :type Integer) (bFromSweep :type Boolean) (SweepResult :type "HitResult Structure (by ref)"))
  (bind _returnvalue (`AIBlueprintHelperLibrary.GetAIController` self))
  (bind _ascannon_controller (cast `/Game/Game/Turret/Cannon/Cannon_Controller` _returnvalue))
  (`/Game/Game/Turret/Cannon/Cannon_Controller.SetTarget` _ascannon_controller OtherActor))

(event `self.ReachRadius.OnComponentEndOverlap`
  (params (OverlappedComponent :type "PrimitiveComponent Object Reference") (OtherActor :type "Actor Object Reference") (OtherComp :type "PrimitiveComponent Object Reference") (OtherBodyIndex :type Integer))
  (bind _overlappingactors (`PrimitiveComponent.GetOverlappingActors` (`self.ReachRadius`) null))
  (bind _returnvalue (`AIBlueprintHelperLibrary.GetAIController` self))
  (bind _ascannon_controller (cast `/Game/Game/Turret/Cannon/Cannon_Controller` _returnvalue))
  (`/Game/Game/Turret/Cannon/Cannon_Controller.EmptyTarget` _ascannon_controller OtherActor)
  (if (>= (`KismetArrayLibrary.Array_Length` _overlappingactors) 1)
    (`/Game/Game/Turret/Cannon/Cannon_Controller.SetTarget` _ascannon_controller (`KismetArrayLibrary.Array_Get` _overlappingactors))))

(event `self.HurtTurret`
  (params (Damage :type "Float (single-precision)"))
  (bind _output_get (set `self.Health` (- (`self.Health`) Damage)))
  (if (<= _output_get 0.0)
    (`self.Kill`)))

(fn `UserConstructionScript`)