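; BP_BuildingSignal is a building placement preview that snaps beside existing buildings and turns red when its body overlaps another actor.
; ConnectorSphere overlaps or Readjust pick the same-class building nearest the controller's mouse position, starting a looping UpdateGrid timer.
; UpdateGrid uses dot products with that partner's axes to offset the preview along world X or Y, flagging snapping on the controller.
; Snapping releases beyond range; Hide parks the actor underground.
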(event `self.ReceiveBeginPlay`
  (bind _asbp_player_controller (cast `/Game/Blueprints/Core/BP_PlayerController` (`GameplayStatics.GetPlayerController` 0)))
  (set `self.CurrentPayerController` _asbp_player_controller))

(event `Hide`
  (`KismetSystemLibrary.K2_SetTimer` self "UpdateGrid" 0.0)
  (`self.K2_SetActorLocation` (0.0 0.0 -10000.0)))

(event `self.ConnectorSphere.OnComponentBeginOverlap`
  (params (OverlappedComponent :type "PrimitiveComponent Object Reference") (OtherActor :type "Actor Object Reference") (OtherComp :type "PrimitiveComponent Object Reference") (OtherBodyIndex :type Integer) (bFromSweep :type Boolean) (SweepResult :type "HitResult Structure (by ref)"))
  (set `self.ClosestBuildingDistance` 1e+18 :!label _label)
  (for _array_element (`PrimitiveComponent.GetOverlappingActors` (`self.ConnectorSphere`) null)
    (bind _asbp_parent_building (cast `/Game/Blueprints/Buildings/BP_ParentBuilding` _array_element))
    (if (== (`GameplayStatics.GetObjectClass` _asbp_parent_building) (`self.CurrentClass`))
      (bind _returnvalue (`KismetMathLibrary.VSize` (- (`/Game/Blueprints/Core/BP_PlayerController.SignalMouseWorldLocation` (`self.CurrentPayerController`)) (`self.K2_GetActorLocation` _asbp_parent_building))))
      (if (< _returnvalue (`self.ClosestBuildingDistance`))
        (set `self.ClosestBuildingDistance` _returnvalue)
        (if (not (== _asbp_parent_building (`self.PartnerBuilding`)))
          (set `self.PartnerBuilding` _asbp_parent_building)
          (`KismetSystemLibrary.K2_SetTimer` self "UpdateGrid" 0.05 true))))))

(event `Readjust`
  (goto _label))

(event `self.Body.OnComponentEndOverlap`
  (params (OverlappedComponent :type "PrimitiveComponent Object Reference") (OtherActor :type "Actor Object Reference") (OtherComp :type "PrimitiveComponent Object Reference") (OtherBodyIndex :type Integer))
  (bind _output_get (set `self.IsOverlapping` (> (`KismetArrayLibrary.Array_Length` (`PrimitiveComponent.GetOverlappingActors` (`self.Body`) null)) 0) :!label _label_2))
  (`self.UpdateHiglightColor` _output_get))

(event `self.Body.OnComponentBeginOverlap`
  (params (OverlappedComponent :type "PrimitiveComponent Object Reference") (OtherActor :type "Actor Object Reference") (OtherComp :type "PrimitiveComponent Object Reference") (OtherBodyIndex :type Integer) (bFromSweep :type Boolean) (SweepResult :type "HitResult Structure (by ref)"))
  (goto _label_2))

(fn `UpdateGrid`
  (bind _defaultsceneroot (`/Game/Blueprints/Buildings/BP_ParentBuilding.DefaultSceneRoot` (`self.PartnerBuilding`)))
  (bind _returnvalue (- (`self.K2_GetActorLocation` (`self.PartnerBuilding`)) (`/Game/Blueprints/Core/BP_PlayerController.SignalMouseWorldLocation` (`self.CurrentPayerController`))))
  (bind _returnvalue_2 (`KismetMathLibrary.Normal` _returnvalue))
  (bind _returnvalue_3 (`KismetMathLibrary.Dot_VectorVector` _returnvalue_2 (`SceneComponent.GetRightVector` _defaultsceneroot)))
  (bind _returnvalue_4 (`KismetMathLibrary.Dot_VectorVector` _returnvalue_2 (`SceneComponent.GetForwardVector` _defaultsceneroot)))
  (bind _returnvalue_5 (`KismetMathLibrary.Abs` _returnvalue_3))
  (if (< (`KismetMathLibrary.VSize` _returnvalue) 200.0)
    (`KismetSystemLibrary.PrintString` (`KismetStringLibrary.Conv_DoubleToString` _returnvalue_3) true true (struct :`G` 0.66 :`B` 1.0 :`A` 1.0) 5.0)
    (if (`KismetMathLibrary.NearlyEqual_FloatFloat` _returnvalue_5 1.0 0.1)
      (`self.K2_SetActorLocation` (+ (`self.K2_GetActorLocation` (`self.PartnerBuilding`)) (`KismetMathLibrary.MakeVector` 0.0 (* (/ _returnvalue_3 _returnvalue_5) (`self.GridPlacementDistance`)))))
      (set `/Game/Blueprints/Core/BP_PlayerController.IsSnappingActive` true (`self.CurrentPayerController`))
      (else
        (`self.K2_SetActorLocation` (+ (`self.K2_GetActorLocation` (`self.PartnerBuilding`)) (`KismetMathLibrary.MakeVector` (* (/ _returnvalue_4 (`KismetMathLibrary.Abs` _returnvalue_4)) (`self.GridPlacementDistance`)))))
        (set `/Game/Blueprints/Core/BP_PlayerController.IsSnappingActive` true (`self.CurrentPayerController`))))
    (else
      (`KismetSystemLibrary.K2_SetTimer` self "UpdateGrid" 0.0)
      (set `/Game/Blueprints/Core/BP_PlayerController.IsSnappingActive` false (`self.CurrentPayerController`))
      (set `self.PartnerBuilding` null))))

(fn `UpdateHiglightColor`
  (params (Red :type Boolean))
  (bind _returnvalue (select `bool` Red :`false` "/Game/Main/Materials/M_Highlight.M_Highlight" :`true` "/Game/Main/Materials/M_RedHighlight.M_RedHighlight" :!type "MaterialInterface Object Reference"))
  (bind _body (`self.Body`))
  (if (!= (`PrimitiveComponent.GetMaterial` _body 0) _returnvalue)
    (`PrimitiveComponent.SetMaterial` _body 0 _returnvalue)
    (`PrimitiveComponent.SetMaterial` (`self.Head`) 0 _returnvalue)
    (`PrimitiveComponent.SetMaterial` (`self.Nozzle`) 0 _returnvalue)))

(fn `UserConstructionScript`)