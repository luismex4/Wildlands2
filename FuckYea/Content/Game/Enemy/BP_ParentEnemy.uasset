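; BP_ParentEnemy is the base class for enemies, providing shared health, damage and death logic.
; Hurt subtracts damage from Health and calls Kill at zero or below, which fires EnemyAmountDecrease before destroying the actor.
; IsDead reports whether Health is depleted.
; NewTarget only prints a debug string here, and the event graph has no active logic.
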(fn `Hurt`
  (params (Damage :type "Float (double-precision)"))
  (bind _output_get (set `self.Health` (- (`self.Health`) Damage)))
  (if (<= _output_get 0.0)
    (`self.Kill`)))

(fn `IsDead`
  (returns (IsDead :type Boolean))
  (return (<= (`self.Health`) 0.0)))

(fn `Kill`
  (`self.EnemyAmountDecrease`)
  (`self.K2_DestroyActor`))

(fn `NewTarget`
  (params (Actor :type "Actor Object Reference"))
  (`KismetSystemLibrary.PrintString` "Called Parent New target"))

(fn `UserConstructionScript`)