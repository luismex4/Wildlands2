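; Rusher enemy character that feeds damage, the Nexus and building or turret targets into its AI blackboard.
; Attack radius overlaps and NewTarget set a building as EnemyTarget, clearing it through that building's death dispatcher.
; Capsule overlaps apply projectile damage with an explosion effect, or target a touched turret.
; Kill decrements the enemy count, ragdolls the mesh, flags IsDead, disables collision and destroys the actor after a delay.
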(event `self.ReceiveBeginPlay`
  (`BlackboardComponent.SetValueAsFloat` (`AIBlueprintHelperLibrary.GetBlackboard` self) "GruntDamage" (`self.Damage`))
  (bind _outactors (`GameplayStatics.GetAllActorsOfClass` "/Game/Blueprints/Buildings/Nexus.Nexus_C"))
  (`BlackboardComponent.SetValueAsObject` (`AIBlueprintHelperLibrary.GetBlackboard` self) "Nexus" (`KismetArrayLibrary.Array_Get` _outactors)))

(event `self.AttackRadius.OnComponentBeginOverlap`
  (params (OverlappedComponent :type "PrimitiveComponent Object Reference") (OtherActor :type "Actor Object Reference") (OtherComp :type "PrimitiveComponent Object Reference") (OtherBodyIndex :type Integer) (bFromSweep :type Boolean) (SweepResult :type "HitResult Structure (by ref)"))
  (bind _returnvalue (`AIBlueprintHelperLibrary.GetBlackboard` self))
  (bind _asbp_parent_building (cast `/Game/Blueprints/Buildings/BP_ParentBuilding` OtherActor))
  (`/Engine/EditorBlueprintResources/StandardMacros.IsValid` _returnvalue
    (:`Is Valid`
      (add `/Game/Blueprints/Buildings/BP_ParentBuilding.DeadDispatch` _asbp_parent_building (delegate `TargetBuildingDead`))
      (`BlackboardComponent.SetValueAsObject` _returnvalue "EnemyTarget" _asbp_parent_building))))

(event `TargetBuildingDead`
  (bind _returnvalue (`AIBlueprintHelperLibrary.GetBlackboard` self))
  (`/Engine/EditorBlueprintResources/StandardMacros.IsValid` _returnvalue
    (:`Is Valid`
      (`BlackboardComponent.SetValueAsObject` _returnvalue "EnemyTarget" null))))

(event `self.Kill`
  (`self.EnemyAmountDecrease`)
  (`PrimitiveComponent.SetSimulatePhysics` (`self.Mesh`) true)
  (`BlackboardComponent.SetValueAsBool` (`AIBlueprintHelperLibrary.GetBlackboard` self) "IsDead" true)
  (set `self.IsDead_0` true)
  (`CharacterMovementComponent.SetAvoidanceEnabled` (`self.CharacterMovement`) false)
  (`PrimitiveComponent.SetCollisionEnabled` (`self.CapsuleComponent`) "NoCollision")
  (`KismetSystemLibrary.Delay` 5.0)
  (`self.K2_DestroyActor`))

(event `self.CapsuleComponent.OnComponentBeginOverlap`
  (params (OverlappedComponent :type "PrimitiveComponent Object Reference") (OtherActor :type "Actor Object Reference") (OtherComp :type "PrimitiveComponent Object Reference") (OtherBodyIndex :type Integer) (bFromSweep :type Boolean) (SweepResult :type "HitResult Structure (by ref)"))
  (bind _asprojectile_parent (cast `/Game/Game/Projectiles/ProjectileParent` OtherActor)
    (:`then`
      (`self.Hurt` (`/Game/Game/Projectiles/ProjectileParent.Damage` _asprojectile_parent))
      (`GameplayStatics.SpawnEmitterAtLocation` "/Game/Game/Particles/P_Explosion2.P_Explosion2" (`self.K2_GetActorLocation` _asprojectile_parent))
      (`self.K2_DestroyActor` _asprojectile_parent))
    (:`CastFailed`
      (bind _asbp_parent_turret (cast `/Game/Game/Turret/BP_ParentTurret` OtherActor))
      (if (== OtherComp (`Character.CapsuleComponent` _asbp_parent_turret))
        (`BlackboardComponent.SetValueAsObject` (`AIBlueprintHelperLibrary.GetBlackboard` self) "EnemyTarget" _asbp_parent_turret)))))

(event `self.NewTarget`
  (params (Actor :type "Actor Object Reference"))
  (bind _returnvalue (`AIBlueprintHelperLibrary.GetBlackboard` self))
  (bind _asbp_parent_building (cast `/Game/Blueprints/Buildings/BP_ParentBuilding` Actor))
  (`/Engine/EditorBlueprintResources/StandardMacros.IsValid` _returnvalue
    (:`Is Valid`
      (add `/Game/Blueprints/Buildings/BP_ParentBuilding.DeadDispatch` _asbp_parent_building (delegate `TargetDeath`))
      (`BlackboardComponent.SetValueAsObject` _returnvalue "EnemyTarget" _asbp_parent_building))))

(event `TargetDeath`
  (bind _returnvalue (`AIBlueprintHelperLibrary.GetBlackboard` self))
  (`/Engine/EditorBlueprintResources/StandardMacros.IsValid` _returnvalue
    (:`Is Valid`
      (`BlackboardComponent.SetValueAsObject` _returnvalue "EnemyTarget" null))))

(fn `UserConstructionScript`)