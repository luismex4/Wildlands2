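; Upgrade room actor where a selected turret's head, body and nozzle are swapped on a preview turret held in a child actor.
; Prepare stores the selected turret, finds each part's index in the option arrays and spawns matching parts onto the preview copy.
; The Cycle functions step through each array with wraparound, spawning the new part onto the copy.
; Transfer hands the copy's part actors to the selected turret and clears the copy's references.
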(event `self.ReceiveBeginPlay`
  (bind _asbp_parent_turret (cast `/Game/Game/Turret/BP_ParentTurret` (`ChildActorComponent.ChildActor` (`self.ChildActor`))))
  (set `self.TurretCopy` _asbp_parent_turret))

(fn `CycleBody`
  (params (Addition :type Integer))
  (bind _returnvalue (`KismetArrayLibrary.Array_Length` (`self.BodyOptions`)))
  (bind _output_get (set `self.BodyIndex` (+ Addition (`self.BodyIndex`))))
  (if (>= _output_get _returnvalue)
    (set `self.BodyIndex` 0))
  (if (< _output_get 0)
    (set `self.BodyIndex` (- _returnvalue 1)))
  (bind _returnvalue_2 (`|SpawnActorFromClass` (`KismetArrayLibrary.Array_Get` (`self.BodyOptions`) (`self.BodyIndex`)) (`KismetMathLibrary.MakeTransform` (0.0 0.0 0.0)) "Undefined" "OverrideRootScale"))
  (`/Game/Game/Turret/BP_ParentTurret.SetBodyActor` (`self.TurretCopy`) _returnvalue_2))

(fn `CycleHead`
  (params (IndexAddition :type Integer))
  (bind _returnvalue (`KismetArrayLibrary.Array_Length` (`self.HeadOptions`)))
  (bind _output_get (set `self.HeadIndex` (+ IndexAddition (`self.HeadIndex`))))
  (if (>= _output_get _returnvalue)
    (set `self.HeadIndex` 0))
  (if (< _output_get 0)
    (set `self.HeadIndex` (- _returnvalue 1)))
  (bind _returnvalue_2 (`|SpawnActorFromClass` (`KismetArrayLibrary.Array_Get` (`self.HeadOptions`) (`self.HeadIndex`)) (`KismetMathLibrary.MakeTransform` (0.0 0.0 0.0)) "Undefined" "OverrideRootScale"))
  (`/Game/Game/Turret/BP_ParentTurret.SetHeadActor` (`self.TurretCopy`) _returnvalue_2))

(fn `CycleNozzle`
  (params (Addition :type Integer))
  (bind _returnvalue (`KismetArrayLibrary.Array_Length` (`self.NozzleOptions`)))
  (bind _output_get (set `self.NozzleIndex` (+ Addition (`self.NozzleIndex`))))
  (if (>= _output_get _returnvalue)
    (set `self.NozzleIndex` 0))
  (if (< _output_get 0)
    (set `self.NozzleIndex` (- _returnvalue 1)))
  (bind _returnvalue_2 (`|SpawnActorFromClass` (`KismetArrayLibrary.Array_Get` (`self.NozzleOptions`) (`self.NozzleIndex`)) (`KismetMathLibrary.MakeTransform` (0.0 0.0 0.0)) "Undefined" "OverrideRootScale" null "/Game/Main/Shapes/DestructibleCube.DestructibleCube"))
  (`/Game/Game/Turret/BP_ParentTurret.SetNozzleActor` (`self.TurretCopy`) _returnvalue_2))

(fn `Prepare`
  (params (SelectedTurret :type "/Game/Game/Turret/BP_ParentTurret Object Reference"))
  (locals (TurretCopy2 :type "/Game/Game/Turret/BP_ParentTurret Object Reference"))
  (bind _returnvalue (`GameplayStatics.GetObjectClass` (`/Game/Game/Turret/BP_ParentTurret.BodyActor` (`self.SelectTurret`))))
  (bind _returnvalue_2 (`GameplayStatics.GetObjectClass` (`/Game/Game/Turret/BP_ParentTurret.NozzleActor` (`self.SelectTurret`))))
  (bind _output_get (set `self.SelectTurret` SelectedTurret))
  (for (_array_element _array_index) (`self.HeadOptions`)
    (bind _returnvalue_3 (`GameplayStatics.GetObjectClass` (`/Game/Game/Turret/BP_ParentTurret.HeadActor` _output_get)))
    (if (== _array_element _returnvalue_3)
      (set `self.HeadIndex` _array_index)
      (break)))
  (bind _returnvalue_4 (`|SpawnActorFromClass` _returnvalue_3 (`KismetMathLibrary.MakeTransform` (0.0 0.0 0.0)) "Undefined" "OverrideRootScale"))
  (`/Game/Game/Turret/BP_ParentTurret.SetHeadActor` (`self.TurretCopy`) _returnvalue_4)
  (for (_array_element_2 _array_index_2) (`self.BodyOptions`)
    (if (== _array_element_2 _returnvalue)
      (set `self.BodyIndex` _array_index_2)
      (break)))
  (bind _returnvalue_5 (`|SpawnActorFromClass` _returnvalue (`KismetMathLibrary.MakeTransform` (0.0 0.0 0.0)) "Undefined" "OverrideRootScale"))
  (`/Game/Game/Turret/BP_ParentTurret.SetBodyActor` (`self.TurretCopy`) _returnvalue_5)
  (for (_array_element_3 _array_index_3) (`self.NozzleOptions`)
    (if (== _array_element_3 _returnvalue_2)
      (set `self.NozzleIndex` _array_index_3)
      (break)))
  (bind _returnvalue_6 (`|SpawnActorFromClass` _returnvalue_2 (`KismetMathLibrary.MakeTransform` (0.0 0.0 0.0)) "Undefined" "OverrideRootScale" null "/Game/Main/Shapes/DestructibleCube.DestructibleCube"))
  (`/Game/Game/Turret/BP_ParentTurret.SetNozzleActor` (`self.TurretCopy`) _returnvalue_6))

(fn `Transfer`
  (`/Game/Game/Turret/BP_ParentTurret.SetHeadActor` (`self.SelectTurret`) (`/Game/Game/Turret/BP_ParentTurret.HeadActor` (`self.TurretCopy`)))
  (`/Game/Game/Turret/BP_ParentTurret.SetBodyActor` (`self.SelectTurret`) (`/Game/Game/Turret/BP_ParentTurret.BodyActor` (`self.TurretCopy`)))
  (`/Game/Game/Turret/BP_ParentTurret.SetNozzleActor` (`self.SelectTurret`) (`/Game/Game/Turret/BP_ParentTurret.NozzleActor` (`self.TurretCopy`)))
  (set `/Game/Game/Turret/BP_ParentTurret.NozzleActor` null (`self.TurretCopy`))
  (set `/Game/Game/Turret/BP_ParentTurret.BodyActor` null (`self.TurretCopy`))
  (set `/Game/Game/Turret/BP_ParentTurret.HeadActor` null (`self.TurretCopy`)))

(fn `UserConstructionScript`)