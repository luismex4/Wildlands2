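; BP_RadiusTrail is an effect actor that sweeps a particle trail in a circle of a given Radius around itself.
; From BeginPlay, a fast looping timer yaws the actor, scaled by world delta time, and teleports the particle system to Radius along its forward vector.
; Terminate disables the emitter, then polls on a timer and destroys the actor once no particles remain active.
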(event `self.ReceiveBeginPlay`
  (`KismetSystemLibrary.K2_SetTimerDelegate` (delegate `Translate`) 0.01 true))

(event `Translate`
  (`self.K2_AddActorWorldRotation` (`KismetMathLibrary.MakeRotator` 0.0 0.0 (* (`GameplayStatics.GetWorldDeltaSeconds`) 100.0)))
  (`SceneComponent.K2_SetWorldLocation` (`self.ParticleSystem`) (+ (`self.K2_GetActorLocation`) (* (`self.GetActorForwardVector`) (`self.Radius`))) false true))

(event `Terminate`
  (`ParticleSystemComponent.SetEmitterEnable` (`self.ParticleSystem`) "Particle Emitter" false)
  (`KismetSystemLibrary.K2_SetTimer` self "DestroyWhenInactive" 0.5 true))

(fn `DestroyWhenInactive`
  (if (== (`ParticleSystemComponent.GetNumActiveParticles` (`self.ParticleSystem`)) 0)
    (`self.K2_DestroyActor`)))

(fn `UserConstructionScript`)