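; BP_Sun rotates a directional light to move between day and night, signalling wave and rest-period starts.
; GoToNight and GoToDay add pitch scaled by SunSpeed and delta seconds until near their target angles, then reset their named timers with no time specified.
; Flag-guarded calls start the wave after a short delay at night and the rest period at day.
; Tick applies only a zero rotation.
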(event `StartWave_Delay`
  (`KismetSystemLibrary.Delay` 0.5)
  (`self.Start Wave`))

(event `self.ReceiveTick`
  (params (DeltaSeconds :type "Float (single-precision)"))
  (bind _directionallight (`self.DirectionalLight`))
  (`SceneComponent.K2_SetWorldRotation` _directionallight (`KismetMathLibrary.ComposeRotators` (`SceneComponent.K2_GetComponentRotation` _directionallight)) false false))

(fn `GoToDay`
  (bind _directionallight (`self.DirectionalLight`))
  (bind _returnvalue (`SceneComponent.K2_GetComponentRotation` (`self.DirectionalLight`)))
  (`SceneComponent.K2_SetWorldRotation` _directionallight (`KismetMathLibrary.ComposeRotators` (`SceneComponent.K2_GetComponentRotation` _directionallight) (`KismetMathLibrary.MakeRotator` 0.0 (* (`GameplayStatics.GetWorldDeltaSeconds`) (`self.SunSpeed`)))) false false)
  (if (== _returnvalue (`KismetMathLibrary.MakeRotator` (.roll _returnvalue) -90.0 (.yaw _returnvalue)) :`ErrorTolerance` 1.0)
    (`KismetSystemLibrary.K2_SetTimer` self "GoToDay")
    (if (not (`self.HasRestPeriodStartCalled`))
      (set `self.HasRestPeriodStartCalled` true)
      (`self.RestPeriodStart`))
    (else
      (set `self.HasRestPeriodStartCalled` false))))

(fn `GoToNight`
  (bind _directionallight (`self.DirectionalLight`))
  (bind _returnvalue (`SceneComponent.K2_GetComponentRotation` (`self.DirectionalLight`)))
  (`SceneComponent.K2_SetWorldRotation` _directionallight (`KismetMathLibrary.ComposeRotators` (`SceneComponent.K2_GetComponentRotation` _directionallight) (`KismetMathLibrary.MakeRotator` 0.0 (* (`GameplayStatics.GetWorldDeltaSeconds`) (`self.SunSpeed`)))) false false)
  (if (== _returnvalue (`KismetMathLibrary.MakeRotator` (.roll _returnvalue) 70.0 (.yaw _returnvalue)) :`ErrorTolerance` 1.0)
    (`KismetSystemLibrary.K2_SetTimer` self "GoToNight")
    (if (not (`self.HasWaveStartCalled`))
      (set `self.HasWaveStartCalled` true)
      (`self.StartWave_Delay`))
    (else
      (set `self.HasWaveStartCalled` false))))

(fn `UserConstructionScript`)