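; Base building actor that takes damage, flashes a hurt material and is destroyed when its health runs out.
; The construction script caches the original material of the Building component's first slot.
; Hurt subtracts health and swaps in the hurt material, then either fires a death dispatcher and destroys the actor or sets a short timer to restore the original material.
; IsDead reports whether health is depleted.
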(fn `ChangeBuildingMaterial`
  (params (`New Material` :type "MaterialInterface Object Reference"))
  (`PrimitiveComponent.SetMaterial` (`self.Building`) 0 `New Material`))

(fn `Hurt`
  (params (Damage :type "Float (double-precision)"))
  (bind _output_get (set `self.Health` (- (`self.Health`) Damage)))
  (`self.ChangeBuildingMaterial` (`self.HurtMaterial`))
  (if (<= _output_get 0.0)
    (`self.DeadDispatch`)
    (`self.K2_DestroyActor`)
    (else
      (`KismetSystemLibrary.K2_SetTimer` self "ResetBuildingMaterial" 0.3))))

(fn `IsDead `
  (returns (IsDead :type Boolean))
  (return (<= (`self.Health`) 0.0)))

(fn `ResetBuildingMaterial`
  (`self.ChangeBuildingMaterial` (`self.Original Building Material`)))

(fn `UserConstructionScript`
  (set `self.Original Building Material` (`PrimitiveComponent.GetMaterial` (`self.Building`) 0)))