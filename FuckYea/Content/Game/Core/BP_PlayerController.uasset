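; Player controller for building and managing turrets and buildings, creating the main UI and switching cameras for an upgrade room.
; Space toggles build mode, where a looping timer moves the placement signal to a mouse trace and arrow keys cycle constructs.
; Clicking spawns the construct if unobstructed, then charges its cost or destroys it when unaffordable.
; Outside build mode, clicks select constructs to fill option buttons, with a radius trail for turrets.
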(event `self.ReceiveBeginPlay`
  (`self.InitializeUI`)
  (`self.InitializeVariables`))

(event `Key|LeftMouseButton`
  (params (Key :type "Key Structure" :default "AnyKey"))
  (bind _mainui (`self.MainUI`))
  (:`Pressed`
    (if (and (`self.BuildMode`) (not (`/Game/Game/BP_BuildingSignal.IsOverlapping` (`self.BuildingSignal`))))
      ;[1 1 1] Build
      (bind _returnvalue (`|SpawnActorFromClass` (`KismetArrayLibrary.Array_Get` (`self.AvailableConstructs`) (`self.SelectTurret`)) (`KismetMathLibrary.MakeTransform` (`self.K2_GetActorLocation` (`self.BuildingSignal`))) "Undefined" "OverrideRootScale"))
      (bind _asbp_parent_turret (cast `/Game/Game/Turret/BP_ParentTurret` _returnvalue)
        (:`then`
          (bind _cost (`/Game/Game/Turret/BP_ParentTurret.Cost` _asbp_parent_turret))
          (if (`/Game/Game/UI/W_MainUI.CheckCurrency` _mainui _cost)
            (`/Game/Game/UI/W_MainUI.DecreaseCurrency` _mainui _cost)
            (set `self.IsSnappingActive` false :!label _label)
            (else
              (`self.K2_DestroyActor` _asbp_parent_turret))))
        (:`CastFailed`
          (bind _asbp_parent_building (cast `/Game/Game/Buildings/BP_ParentBuilding` _returnvalue))
          (bind _cost_2 (`/Game/Game/Buildings/BP_ParentBuilding.Cost` _asbp_parent_building))
          (if (`/Game/Game/UI/W_MainUI.CheckCurrency` _mainui _cost_2)
            (`/Game/Game/UI/W_MainUI.DecreaseCurrency` _mainui _cost_2)
            (`/Game/Game/BP_BuildingSignal.Readjust` (`self.BuildingSignal`))
            (goto _label)
            (else
              (`self.K2_DestroyActor` _asbp_parent_building)))))
      (elif (not (`self.BuildMode`))
        (bind (_hitresult _hit_result) (`self.LineTraceMouse`))
        (`|ExecutionSequence`
          (:`then_1`
            (bind (_bblockinghit _binitialoverlap _time _location _impactpoint _normal _impactnormal _physmat _hitactor) (`GameplayStatics.BreakHitResult` _hit_result))
            ;[1 1 1] Select
            (`/Engine/EditorBlueprintResources/StandardMacros.IsValid` _hitactor
              (:`Is Valid`
                (bind _asbp_turret_section (cast `/Game/Game/Turret/BP_TurretSection` _hitactor)
                  (:`then`
                    (bind _parentturret (`/Game/Game/Turret/BP_TurretSection.ParentTurret` _asbp_turret_section))
                    (if (not (== _parentturret (`self.CurrentSelectedTurret`)))
                      (set `self.CurrentSelectedTurret` _parentturret)
                      (`self.ShowSelectedTurretRadius`)
                      (`self.UpdateSelectTurretOptions`)))
                  (:`CastFailed`
                    (bind _asbp_parent_building_2 (cast `/Game/Game/Buildings/BP_ParentBuilding` _hitactor :!label _label_2)
                      (:`then`
                        (set `self.CurrentSelectedBuilding` _asbp_parent_building_2)
                        (set `self.CurrentSelectedTurret` null)
                        (`self.UpdateSelectBuildingOptions`)
                        (`self.EndRadiusTrail`))
                      (:`CastFailed`
                        ;;[1 1 1] Deselect Current selection
                        (`self.DeselectTurret`))))))
              (:`Is Not Valid`
                (goto _label_2)))))))))

(event `Key|Left`
  (params (Key :type "Key Structure" :default "AnyKey"))
  (:`Pressed`
    (bind _result (`/Engine/EditorBlueprintResources/StandardMacros.DecrementInt` (`self.SelectTurret`))
      (:`  `
        (if (< _result 0)
          (set `self.SelectTurret` (- (`KismetArrayLibrary.Array_Length` (`self.AvailableConstructs`)) 1)))
        (`/Game/Game/UI/W_MainUI.SelectBuildOption` (`self.MainUI`) (`self.SelectTurret`))
        (`/Game/Game/UI/W_MainUI.SelectTurretSwitch` (`self.MainUI`) (`KismetSystemLibrary.GetClassDisplayName` (`KismetArrayLibrary.Array_Get` (`self.AvailableConstructs`) (`self.SelectTurret`))))))))

(event `Key|Right`
  (params (Key :type "Key Structure" :default "AnyKey"))
  (:`Pressed`
    (bind _result (`/Engine/EditorBlueprintResources/StandardMacros.IncrementInt` (`self.SelectTurret`))
      (:`  `
        (if (>= _result (`KismetArrayLibrary.Array_Length` (`self.AvailableConstructs`)))
          (set `self.SelectTurret` 0))
        (`/Game/Game/UI/W_MainUI.SelectBuildOption` (`self.MainUI`) (`self.SelectTurret`))
        (`/Game/Game/UI/W_MainUI.SelectTurretSwitch` (`self.MainUI`) (`KismetSystemLibrary.GetClassDisplayName` (`KismetArrayLibrary.Array_Get` (`self.AvailableConstructs`) (`self.SelectTurret`))))))))

(event `Key|SpaceBar`
  (params (Key :type "Key Structure" :default "AnyKey"))
  (:`Pressed`
    (`self.DeselectTurret`)
    (bind _output_get (set `self.BuildMode` (not (`self.BuildMode`))))
    (if _output_get
      (`/Game/Game/UI/W_MainUI.SetMode` (`self.MainUI`) "NewEnumerator1")
      (`KismetSystemLibrary.K2_SetTimer` self "ShowBuildingSignal" 0.05 true)
      (else
        (`/Game/Game/UI/W_MainUI.SetMode` (`self.MainUI`) "NewEnumerator0")
        (`KismetSystemLibrary.K2_SetTimer` self "ShowBuildingSignal")
        (set `self.IsSnappingActive` false)
        (`/Game/Game/BP_BuildingSignal.Hide` (`self.BuildingSignal`))))))

(fn `ChangeSelectConstruct`
  (params (Index :type Integer))
  (bind _output_get (set `self.SelectTurret` Index))
  (if (>= _output_get (`KismetArrayLibrary.Array_Length` (`self.AvailableConstructs`)))
    (set `self.SelectTurret` 0))
  (`/Game/Game/UI/W_MainUI.SelectTurretSwitch` (`self.MainUI`) (`KismetSystemLibrary.GetClassDisplayName` (`KismetArrayLibrary.Array_Get` (`self.AvailableConstructs`) (`self.SelectTurret`)))))

(fn `DeselectTurret`
  (`/Engine/EditorBlueprintResources/StandardMacros.IsValid` (`self.CurrentSelectedTurret`)
    (:`Is Valid`
      (`/Game/Game/UI/W_MainUI.HideConstructOptions` (`self.MainUI`))
      (`self.EndRadiusTrail`)
      (set `self.CurrentSelectedTurret` null))))

(fn `EndRadiusTrail`
  (bind _currentraidustrail (`self.CurrentRaidusTrail`))
  (`/Engine/EditorBlueprintResources/StandardMacros.IsValid` _currentraidustrail
    (:`Is Valid`
      (`/Game/Game/FX/BP_RadiusTrail.Terminate` _currentraidustrail))))

(fn `Find Mouse to Land Distance`
  (bind (_worldlocation _worlddirection) (`self.DeprojectMousePositionToWorld`))
  (bind _outhit (`KismetSystemLibrary.LineTraceSingle` _worldlocation (+ _worldlocation (* _worlddirection 3000.0)) "TraceTypeQuery1" false (`|MakeArray` (`self.BuildingSignal`) :!type "Actor Object Reference") "Persistent" true (struct :`R` 1.0 :`A` 1.0) (struct :`R` 1.0 :`A` 1.0)))
  (bind (_bblockinghit _binitialoverlap _time _location _impactpoint _normal _impactnormal _physmat _hitactor) (`GameplayStatics.BreakHitResult` _outhit))
  (cast `Landscape` _hitactor)
  (set `self.MouseToLandDistance` (`KismetMathLibrary.VSize` (- _location _worldlocation)))
  (`KismetSystemLibrary.K2_SetTimer` self "Find Mouse to Land Distance" 0.0))

(fn `InitializeUI`
  (bind _returnvalue (`|CreateWidget` "/Game/Game/UI/W_MainUI.W_MainUI_C"))
  (bind _output_get (set `self.MainUI` _returnvalue))
  (`UserWidget.AddToViewport` _output_get 0))

(fn `InitializeVariables`
  (bind _outactors (`GameplayStatics.GetAllActorsOfClass` "/Game/Game/BP_BuildingSignal.BP_BuildingSignal_C"))
  (set `self.BuildingSignal` (`KismetArrayLibrary.Array_Get` _outactors))
  (bind _outactors_2 (`GameplayStatics.GetAllActorsOfClass` "/Game/Game/Upgrade/BP_UpgradeRoom.BP_UpgradeRoom_C"))
  (set `self.UpgradeRoom` (`KismetArrayLibrary.Array_Get` _outactors_2))
  (bind _outactors_3 (`GameplayStatics.GetAllActorsWithTag` "SceneCamera"))
  (bind _ascamera_actor (cast `CameraActor` (`KismetArrayLibrary.Array_Get` _outactors_3)))
  (set `self.SceneCamera` _ascamera_actor))

(fn `LineTraceMouse`
  (returns (HitResult :type Boolean) (`Hit Result` :type "HitResult Structure"))
  (bind (_worldlocation _worlddirection) (`self.DeprojectMousePositionToWorld`))
  (bind (_outhit _returnvalue) (`KismetSystemLibrary.LineTraceSingle` _worldlocation (+ _worldlocation (* _worlddirection 3000.0)) "TraceTypeQuery1" false (`|MakeArray` (`self.BuildingSignal`) :!type "Actor Object Reference") "None" true (struct :`R` 1.0 :`A` 1.0) (struct :`R` 1.0 :`A` 1.0)))
  (return _returnvalue _outhit))

(fn `Reposition`)

(fn `ShowBuildingSignal`
  (if (`self.BuildMode`)
    (bind (_hitresult _hit_result) (`self.LineTraceMouse`))
    (bind _output_get (set `self.SignalMouseWorldLocation` (`.Location` (`GameplayStatics.BreakHitResult` _hit_result))))
    (if (not (`self.IsSnappingActive`))
      (`self.K2_SetActorLocation` (`self.BuildingSignal`) _output_get false true))
    (else
      (`/Game/Game/BP_BuildingSignal.Hide` (`self.BuildingSignal`)))))

(fn `ShowSelectedTurretRadius`
  (bind _currentselectedturret (`self.CurrentSelectedTurret`))
  (bind _currentraidustrail (`self.CurrentRaidusTrail`))
  (bind _returnvalue (`self.K2_GetActorLocation` _currentselectedturret))
  (bind _returnvalue_2 (`SphereComponent.GetScaledSphereRadius` (`/Game/Game/Turret/BP_ParentTurret.ReachRadius` _currentselectedturret)))
  (`/Engine/EditorBlueprintResources/StandardMacros.IsValid` (`self.CurrentRaidusTrail`)
    (:`Is Valid`
      (`self.K2_SetActorLocation` _currentraidustrail _returnvalue false false)
      (set `/Game/Game/FX/BP_RadiusTrail.Radius` _returnvalue_2 _currentraidustrail))
    (:`Is Not Valid`
      (bind _returnvalue_3 (`|SpawnActorFromClass` "/Game/Game/FX/BP_RadiusTrail.BP_RadiusTrail_C" (`KismetMathLibrary.MakeTransform` _returnvalue) "Undefined" "OverrideRootScale" null _returnvalue_2))
      (set `self.CurrentRaidusTrail` _returnvalue_3))))

(fn `SwitchToNormalMode`
  (`self.SetViewTargetWithBlend` (`self.SceneCamera`))
  (`WidgetSwitcher.SetActiveWidgetIndex` (`/Game/Game/UI/W_MainUI.WidgetSwitcher_0` (`self.MainUI`)) 0))

(fn `SwitchToUpgradeMode`
  (`/Game/Game/Upgrade/BP_UpgradeRoom.Prepare` (`self.UpgradeRoom`) (`self.CurrentSelectedTurret`))
  (`self.SetViewTargetWithBlend` (`self.UpgradeRoom`) 0.0)
  (`WidgetSwitcher.SetActiveWidgetIndex` (`/Game/Game/UI/W_MainUI.WidgetSwitcher_0` (`self.MainUI`)) 1))

(fn `UpdateSelectBuildingOptions`
  (`/Game/Game/UI/W_MainUI.ClearConstructOptions` (`self.MainUI`))
  (bind _returnvalue (`|CreateWidget` "/Game/Game/UI/W_ConstructOptionsButton.W_ConstructOptionsButton_C" null null (`self.CurrentSelectedBuilding`) "NewEnumerator2" self (`self.MainUI`)))
  (`/Game/Game/UI/W_MainUI.AddConstructOption` (`self.MainUI`) _returnvalue)
  (bind _returnvalue_2 (`|CreateWidget` "/Game/Game/UI/W_ConstructOptionsButton.W_ConstructOptionsButton_C" null null (`self.CurrentSelectedBuilding`) "NewEnumerator2" self (`self.MainUI`)))
  (`/Game/Game/UI/W_MainUI.AddConstructOption` (`self.MainUI`) _returnvalue_2)
  (bind _returnvalue_3 (`|CreateWidget` "/Game/Game/UI/W_ConstructOptionsButton.W_ConstructOptionsButton_C" null null (`self.CurrentSelectedBuilding`) "NewEnumerator2" self (`self.MainUI`)))
  (`/Game/Game/UI/W_MainUI.AddConstructOption` (`self.MainUI`) _returnvalue_3)
  (bind _returnvalue_4 (`|CreateWidget` "/Game/Game/UI/W_ConstructOptionsButton.W_ConstructOptionsButton_C" null null (`self.CurrentSelectedBuilding`) "NewEnumerator2" self (`self.MainUI`)))
  (`/Game/Game/UI/W_MainUI.AddConstructOption` (`self.MainUI`) _returnvalue_4)
  (`/Game/Game/UI/W_MainUI.ShowConstructOptions` (`self.MainUI`)))

(fn `UpdateSelectTurretOptions`
  (`|ExecutionSequence`
    (:`then_0`
      (`/Game/Game/UI/W_MainUI.ClearConstructOptions` (`self.MainUI`))
      (bind _returnvalue (`|CreateWidget` "/Game/Game/UI/W_ConstructOptionsButton.W_ConstructOptionsButton_C" null (`self.CurrentSelectedTurret`) null "NewEnumerator2" self (`self.MainUI`)))
      (`/Game/Game/UI/W_MainUI.AddConstructOption` (`self.MainUI`) _returnvalue)
      (bind _returnvalue_2 (`|CreateWidget` "/Game/Game/UI/W_ConstructOptionsButton.W_ConstructOptionsButton_C" null (`self.CurrentSelectedTurret`) null "NewEnumerator1" self (`self.MainUI`)))
      (`/Game/Game/UI/W_MainUI.AddConstructOption` (`self.MainUI`) _returnvalue_2))
    (:`then_1`
      (`/Game/Game/UI/W_MainUI.ShowConstructOptions` (`self.MainUI`)))))

(fn `UserConstructionScript`)