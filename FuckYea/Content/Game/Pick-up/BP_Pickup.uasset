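; BP_Pickup is an upgrade pickup that randomly becomes a Head, Nozzle or Body part.
; BeginPlay rolls the part type from the enum, picks a mesh from that type's upgrade array, then plays a Spawn timeline that animates the instanced static mesh's relative location.
; CreatePartData packages the mesh and type as upgrade data, with zeroed stats and a placeholder name.
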(event `self.ReceiveBeginPlay`
  (bind _headupgrades (`self.HeadUpgrades`))
  (bind _bodyupgrades (`self.BodyUpgrades`))
  (bind _nozzleupgrades (`self.NozzleUpgrades`))
  (`|ExecutionSequence`
    (:`then_0`
      (set `self.MeshType` (cast `/Game/Game/Data/E_PartType` (`KismetMathLibrary.Conv_IntToByte` (`KismetMathLibrary.RandomIntegerInRange` 0 (- (enumcount `/Game/Game/Data/E_PartType`) 1)))))
      (switch `/Game/Game/Data/E_PartType` (`self.MeshType`)
        (:`NewEnumerator0`
          (set `self.Mesh` (`KismetArrayLibrary.Array_Get` _headupgrades (`KismetMathLibrary.RandomIntegerInRange` 0 (- (`KismetArrayLibrary.Array_Length` _headupgrades) 1)))))
        (:`NewEnumerator1`
          (set `self.Mesh` (`KismetArrayLibrary.Array_Get` _nozzleupgrades (`KismetMathLibrary.RandomIntegerInRange` 0 (- (`KismetArrayLibrary.Array_Length` _nozzleupgrades) 1)))))
        (:`NewEnumerator3`
          (set `self.Mesh` (`KismetArrayLibrary.Array_Get` _bodyupgrades (`KismetMathLibrary.RandomIntegerInRange` 0 (- (`KismetArrayLibrary.Array_Length` _bodyupgrades) 1)))))))
    (:`then_1`
      (bind (_direction _offset) (`Timeline|Spawn`)
        (:`Update`
          (`SceneComponent.K2_SetRelativeLocation` (`self.InstancedStaticMesh`) (* _offset 300.0) false false))))))

(fn `CreatePartData`
  (returns (UpgradeData :type "/Game/Game/Data/S_UpgradeData Structure"))
  (return (make `/Game/Game/Data/S_UpgradeData` (`self.Mesh`) (`self.MeshType`) 0.0 0.0 0.0 0.0 "Test")))

(fn `UserConstructionScript`)